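; Player controller for a Control4 test that lets the player switch between four top-down characters.
; On BeginPlay, if the Enhanced Input subsystem is valid, it adds the Control4 mapping context and caches every BP_TopDownCharacter in the level.
; The Q, W, E and R input actions each possess one of the first four cached characters, indexed directly in the order GetAllActorsOfClass returns them.
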(event Input|EnhancedActionEvents|EnhancedInputActionIA_Q
  (params (ActionValue :type Boolean) (ElapsedSeconds :type Float%20%28double-precision%29) (TriggeredSeconds :type Float%20%28double-precision%29) (InputAction :type Input%20Action%20Object%20Reference :default "/Game/Control4_3D_Test/Input/Actions/IA_Q.IA_Q"))
  (:Started
    (Pawn|Possess (Utilities|Array|Get(acopy) (Variables|Default|GetCharacters)))))

(event Input|EnhancedActionEvents|EnhancedInputActionIA_W
  (params (ActionValue :type Boolean) (ElapsedSeconds :type Float%20%28double-precision%29) (TriggeredSeconds :type Float%20%28double-precision%29) (InputAction :type Input%20Action%20Object%20Reference :default "/Game/Control4_3D_Test/Input/Actions/IA_W.IA_W"))
  (:Started
    (Pawn|Possess (Utilities|Array|Get(acopy) (Variables|Default|GetCharacters) 1))))

(event Input|EnhancedActionEvents|EnhancedInputActionIA_E
  (params (ActionValue :type Boolean) (ElapsedSeconds :type Float%20%28double-precision%29) (TriggeredSeconds :type Float%20%28double-precision%29) (InputAction :type Input%20Action%20Object%20Reference :default "/Game/Control4_3D_Test/Input/Actions/IA_E.IA_E"))
  (:Started
    (Pawn|Possess (Utilities|Array|Get(acopy) (Variables|Default|GetCharacters) 2))))

(event Input|EnhancedActionEvents|EnhancedInputActionIA_R
  (params (ActionValue :type Boolean) (ElapsedSeconds :type Float%20%28double-precision%29) (TriggeredSeconds :type Float%20%28double-precision%29) (InputAction :type Input%20Action%20Object%20Reference :default "/Game/Control4_3D_Test/Input/Actions/IA_R.IA_R"))
  (:Started
    (Pawn|Possess (Utilities|Array|Get(acopy) (Variables|Default|GetCharacters) 3))))

(event EventBeginPlay
  (bind _returnvalue (PlayerController|LocalPlayerSubsystems|GetEnhancedInputLocalPlayerSubsystem))
  (Utilities|IsValid _returnvalue
    (:Is%20Valid
      (Input|AddMappingContext _returnvalue "/Game/Control4_3D_Test/Input/IMC_Control4.IMC_Control4" 0 "(bIgnoreAllPressedKeysUntilRelease=True,bForceImmediately=False)")
      (bind _outactors (Actor|GetAllActorsOfClass "/Game/TopDown/Blueprints/BP_TopDownCharacter.BP_TopDownCharacter_C"))
      (Variables|Default|SetCharacters _outactors))))

(event EventTick
  (params (DeltaSeconds :type Float%20%28single-precision%29)))

(fn ConstructionScript
  (|CallParentFunction))